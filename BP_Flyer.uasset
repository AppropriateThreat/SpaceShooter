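; BP_Flyer is a flyer Blueprint with two Niagara thruster effects on its PlayerModel.
; BeginPlay attaches both effects at the thruster1 and thruster2 attach points and stores references to them.
; Each Tick, UpdateThrusters writes their User.AttractorPosition parameter.
; Only the first thruster's X comes from a clamped range mapping, whose inputs are unset; the second receives no computed value.
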(event EventBeginPlay
  (bind _returnvalue (Niagara|SpawnSystemAttached "/Game/assets/ThrusterEmitter_System.ThrusterEmitter_System" (Variables|Default|GetPlayerModel) "thruster1" "0, 0, 0" "0, 0, 0" "SnapToTargetIncludingScale" false))
  (Variables|Default|Setthruster1FXs _returnvalue)
  (bind _returnvalue_2 (Niagara|SpawnSystemAttached "/Game/assets/ThrusterEmitter_System.ThrusterEmitter_System" (Variables|Default|GetPlayerModel) "thruster2" "0, 0, 0" "0, 0, 0" "SnapToTargetIncludingScale" false))
  (Variables|Default|Setthruster2FXS _returnvalue_2))

(event Collision|EventActorBeginOverlap
  (params (OtherActor :type Actor%20Object%20Reference)))

(event EventTick
  (params (DeltaSeconds :type Float%20%28single-precision%29))
  (CallFunction|UpdateThrusters))

(fn ConstructionScript)

(fn UpdateThrusters
  (Niagara|SetNiagaraVariable(Vector3) (Variables|Default|Getthruster1FXs) "User.AttractorPosition" (Math|Vector|MakeVector (Math|Float|MapRangeClamped 0.0 0.0 0.0 0.0 0.0) 0.0 0.0))
  (Niagara|SetNiagaraVariable(Vector3) (Variables|Default|Getthruster2FXS) "User.AttractorPosition" (Math|Vector|MakeVector 0.0 0.0 0.0)))